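; BP_ProjectileVFXSPawner is an actor that repeatedly fires Niagara projectile effects from its own location.
; On BeginPlay it spawns one BP_ProjectileManager immediately, then repeats on a looping timer at a configurable interval.
; Each spawned projectile receives the spawner's muzzle, main and hit effects, an X-axis velocity, hit offset and destroy delay.
; It also pushes the trail loop duration into the projectile's Niagara user variable.
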(event Custom|Spawn%20Projectile%20VFX
  (bind _returnvalue (Game|SpawnActorfromClass "/Game/Niagara/BP_Spawner/BP_ProjectileManager.BP_ProjectileManager_C" (Math|Transform|MakeTransform (Transformation|GetActorLocation) "0, 0, 0" "1.000000,1.000000,1.000000") "Undefined" "MultiplyWithRoot" 0 0))
  (bind _output_get (Variables|Default|SetSpawnedProjectile _returnvalue))
  (Utilities|IsValid _output_get
    (:Is%20Valid
      (Utilities|FlowControl|Sequence
        (:then_0
          (Variables|/Game/Niagara/BP_Spawner/BP_ProjectileManager.BP_ProjectileManager_C|SetMuzzleVFX (Variables|Default|GetSpawnedProjectile) (Variables|Default|GetMuzzleVFX))
          (Class|NiagaraComponent|SetAsset (Variables|/Game/Niagara/BP_Spawner/BP_ProjectileManager.BP_ProjectileManager_C|GetProjectile%20VFX (Variables|Default|GetSpawnedProjectile)) (Variables|Default|GetMainProjectileVFX) true)
          (Variables|/Game/Niagara/BP_Spawner/BP_ProjectileManager.BP_ProjectileManager_C|SetHitVFX (Variables|Default|GetSpawnedProjectile) (Variables|Default|GetHit%20VFX)))
        (:then_1
          (Variables|/Script/Engine.MovementComponent|SetVelocity (Variables|/Game/Niagara/BP_Spawner/BP_ProjectileManager.BP_ProjectileManager_C|GetProjectileVFXMovement (Variables|Default|GetSpawnedProjectile)) (* (Variables|Default|GetProjectile%20Speed) "1.000000,0.000000,0.000000")))
        (:then_2
          (Variables|/Game/Niagara/BP_Spawner/BP_ProjectileManager.BP_ProjectileManager_C|SetMuzzleHitOffset (Variables|Default|GetSpawnedProjectile) (Variables|Default|GetMuzzle%20Hit%20Offset))
          (Variables|/Game/Niagara/BP_Spawner/BP_ProjectileManager.BP_ProjectileManager_C|SetDestroyDelay (Variables|Default|GetSpawnedProjectile) (Variables|Default|GetDestroy%20Delay))
          (Niagara|SetNiagaraVariable(Float) (Variables|/Game/Niagara/BP_Spawner/BP_ProjectileManager.BP_ProjectileManager_C|GetProjectile%20VFX (Variables|Default|GetSpawnedProjectile)) "TrailLoopDuration" (Variables|Default|GetTrailLoopDuration)))))))

(event EventBeginPlay
  (CallFunction|SpawnProjectileVFX)
  (Utilities|Time|SetTimerbyEvent (delegate Custom|Spawn%20Projectile%20VFX) (Variables|Default|GetProjectile%20Spawn%20Interval) true))

(fn ConstructionScript)